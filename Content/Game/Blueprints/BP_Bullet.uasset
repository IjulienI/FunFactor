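; BP_Bullet is an explosive projectile that deals radial damage when it touches something.
; On spawn it attaches a trail effect and starts a timed self-destruct.
; Each tick it runs a zero-length sphere trace at its own position on the Visibility channel, ignoring the player character.
; A hit spawns a random explosion emitter, draws a debug blast sphere, applies radial damage, shakes nearby cameras and destroys the bullet.
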(event EventBeginPlay
  (Niagara|SpawnSystemAttached "/Game/Game/VFX/VFX_Trail.VFX_Trail" (Variables|Default|GetSphere) "None" "0, 0, 0" "0, 0, 0" "KeepRelativeOffset" false)
  (Utilities|FlowControl|Delay 35.0)
  (Actor|DestroyActor))

(event EventTick
  (params (DeltaSeconds :type Float%20%28single-precision%29))
  (bind _sphere (Variables|Default|GetSphere))
  (bind _sphere_2 (Variables|Default|GetSphere))
  (bind _returnvalue (Transformation|GetWorldLocation _sphere_2))
  (bind _returnvalue_2 (Transformation|GetWorldLocation _sphere))
  (bind _asbp_first_person_character (Utilities|Casting|CastToBP_FirstPersonCharacter (Game|Player|GetPlayerPawn 0)))
  (bind (_outhit _returnvalue_3) (Collision|SphereTraceByChannel _returnvalue _returnvalue 15.0 "TraceTypeQuery1" true (Utilities|Array|MakeArray _asbp_first_person_character) "None"))
  (if _returnvalue_3
    (Effects|SpawnEmitteratLocation (.OutItem (Utilities|Array|Random (Variables|Default|GetEmitter%20Template))) _returnvalue_2 "0, 0, 0" "3.000000,3.000000,3.000000")
    (Rendering|Debug|DrawDebugSphere _returnvalue_2 2.5e+02 12 "(R=1.000000,G=0.042102,B=0.000000,A=1.000000)" 2.0)
    (Game|Damage|ApplyRadialDamage 2.5e+02 _returnvalue_2 2.5e+02 0 0 0 0 false "ECC_Visibility")
    (Camera|PlayWorldCameraShake "/Game/Game/Character/BP_Shake.BP_Shake_C" (Transformation|GetWorldLocation (Variables|Default|GetSphere)) 1.5e+02 5e+03 0.5)
    (Actor|DestroyActor)))

(fn ConstructionScript)
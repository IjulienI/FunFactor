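; BP_Damage is a short-lived actor that shows a damage number in the world.
; One tick after BeginPlay it passes AmountDamage to its WBP_ShowDamage widget, scales its static mesh by that amount and launches the mesh with a random impulse.
; It destroys itself after a one-second delay, and every tick turns the widget toward the first-person character's mesh.
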(event Collision|EventActorBeginOverlap
  (params (OtherActor :type Actor%20Object%20Reference)))

(event EventTick
  (params (DeltaSeconds :type Float%20%28single-precision%29))
  (bind _asbp_first_person_character (Utilities|Casting|CastToBP_FirstPersonCharacter (Game|Player|GetPlayerPawn 0)))
  (Transformation|SetWorldRotation (Variables|Default|GetWidget) (Math|Rotator|FindLookatRotation (Transformation|GetWorldLocation (Variables|Default|GetWidget)) (Transformation|GetWorldLocation (Variables|/Script/Engine.Character|GetMesh _asbp_first_person_character))) false false))

(event EventBeginPlay
  (bind _amountdamage (Variables|Default|GetAmountDamage))
  (Utilities|FlowControl|DelayUntilNextTick)
  (bind _aswbp_show_damage (Utilities|Casting|CastToWBP_ShowDamage (UserInterface|GetUserWidgetObject (Variables|Default|GetWidget))))
  (Default|SetText _aswbp_show_damage _amountdamage)
  (Transformation|SetRelativeScale3D (Variables|Default|GetStaticMesh) (Math|Conversions|ToVector(Float) (* _amountdamage 0.01)))
  (Physics|AddImpulse (Variables|Default|GetStaticMesh) (Math|Vector|MakeVector (Math|Random|RandomFloatinRange -6e+02 6e+02) (Math|Random|RandomFloatinRange -6e+02 6e+02) (Math|Random|RandomFloatinRange -6e+02 6e+02)) "None" true)
  (Utilities|FlowControl|Delay 1.0)
  (Actor|DestroyActor))

(fn ConstructionScript)